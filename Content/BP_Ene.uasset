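; BP_Ene is an enemy character that shoots bullets and whose death ends the game.
; AnyDamage drains Energy2; at zero it briefly shows the BP_WEnd widget, then destroys the actor and calls QuitGame.
; AttackTo spawns BP_Bullet at Arrow1, while Run, Walk and Ready set movement speed or halt it.
; SetState is an empty stub with an unconnected switch, and nothing in this file calls the action functions.
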(event `self.ReceiveAnyDamage`
  (params (Damage :type "Float (single-precision)") (DamageType :type "DamageType Object Reference") (InstigatedBy :type "Controller Object Reference") (DamageCauser :type "Actor Object Reference"))
  (bind _output_get (set `self.Energy2` (- (`self.Energy2`) Damage)))
  (if (<= _output_get 0.0)
    (bind _returnvalue (`|CreateWidget` "/Game/BP_WEnd.BP_WEnd_C"))
    (`UserWidget.AddToViewport` _returnvalue 0)
    (`KismetSystemLibrary.Delay` 3.0)
    (`Widget.RemoveFromParent` _returnvalue)
    (`KismetSystemLibrary.Delay` 1.0)
    (`self.K2_DestroyActor`)
    (`KismetSystemLibrary.QuitGame` null "Quit")))

(fn `attack to`
  (`|SpawnActorFromClass` "/Game/BP_Bullet.BP_Bullet_C" (`SceneComponent.K2_GetComponentToWorld` (`self.Arrow1`)) "Undefined" "OverrideRootScale" null null))

(fn `ready`
  (bind _charactermovement (`self.CharacterMovement`))
  (set `MovementComponent.Velocity` (0.0 0.0 0.0) _charactermovement)
  (set `CharacterMovementComponent.MaxWalkSpeed` 0.0 _charactermovement))

(fn `run`
  (set `CharacterMovementComponent.MaxWalkSpeed` 330.0 (`self.CharacterMovement`)))

(fn `SetState `
  (params (state :type Integer)))

(fn `UserConstructionScript`
  (`parent.UserConstructionScript`))

(fn `Walk`
  (set `self.Is Shot2` false)
  (set `CharacterMovementComponent.MaxWalkSpeed` 230.0 (`self.CharacterMovement`)))