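; AI controller for BP_Ene enemies that runs behavior tree BT_A and supplies its blackboard data.
; On BeginPlay it writes the pawn's two point locations as spot keys.
; Perception updates toggle the player key for actors tagged Player, clearing it if already set.
; Every Tick it refreshes player location, distance, a close-range flag and whether the enemy has energy left.
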(event `self.ReceiveBeginPlay`
  (`self.RunBehaviorTree` "/Game/BT_A.BT_A")
  (`self.IniSpot`))

(event `self.AIPerception.OnPerceptionUpdated`
  (params (UpdatedActors :type "Array of Actor Object Reference (by ref)"))
  (for _array_element UpdatedActors
    (`self.Player Existence` _array_element)))

(event `self.ReceiveTick`
  (params (DeltaSeconds :type "Float (single-precision)"))
  (`self.UpdateVec`))

(fn `IniSpot`
  (bind _asbp_ene (cast `/Game/BP_Ene` (`self.K2_GetPawn`)))
  (`BlackboardComponent.SetValueAsVector` (`AIBlueprintHelperLibrary.GetBlackboard` null) "SpotKey" (`self.K2_GetActorLocation` (`/Game/BP_Ene.Point1` _asbp_ene)))
  (`BlackboardComponent.SetValueAsVector` (`AIBlueprintHelperLibrary.GetBlackboard` null) "SpotKey2" (`self.K2_GetActorLocation` (`/Game/BP_Ene.Point2` _asbp_ene))))

(fn `Player Existence`
  (params (`player exist` :type "Actor Object Reference"))
  (if (`self.ActorHasTag` `player exist` "Player")
    (`/Engine/EditorBlueprintResources/StandardMacros.IsValid` (`BlackboardComponent.GetValueAsObject` (`AIBlueprintHelperLibrary.GetBlackboard` null) "PlayerKey")
      (:`Is Valid`
        (`BlackboardComponent.SetValueAsObject` (`AIBlueprintHelperLibrary.GetBlackboard` null) "PlayerKey" null))
      (:`Is Not Valid`
        (`BlackboardComponent.SetValueAsObject` (`AIBlueprintHelperLibrary.GetBlackboard` null) "PlayerKey" `player exist`)))))

(fn `UpdateVec`
  (bind _asbp_ene (cast `/Game/BP_Ene` (`self.K2_GetPawn`)))
  (bind _asbp_cha (cast `/Game/BP_Cha` (`GameplayStatics.GetPlayerCharacter` 0)))
  (bind _returnvalue (`self.K2_GetActorLocation` _asbp_cha))
  (`BlackboardComponent.SetValueAsVector` (`AIBlueprintHelperLibrary.GetBlackboard` null) "PlayerLocationKey" _returnvalue)
  (bind _returnvalue_2 (`KismetMathLibrary.VSize` (- (`self.K2_GetActorLocation` _asbp_ene) _returnvalue)))
  (`BlackboardComponent.SetValueAsFloat` (`AIBlueprintHelperLibrary.GetBlackboard` null) "DistKey" _returnvalue_2)
  (`BlackboardComponent.SetValueAsBool` (`AIBlueprintHelperLibrary.GetBlackboard` null) "RangeKey" (<= _returnvalue_2 150.0))
  (`BlackboardComponent.SetValueAsBool` (`AIBlueprintHelperLibrary.GetBlackboard` null) "EnergyKey" (> (`/Game/BP_Ene.Energy2` _asbp_ene) 0.0)))

(fn `UserConstructionScript`)