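; Player character Blueprint with forward movement, yaw turning, a held-button run and bullet shooting.
; Shooting is allowed only while standing still; it sets IsShot and spawns a BP_Bullet at the Arrow1 transform.
; Damage drains Energy; at zero it disables input, shows the BP_WEnd widget briefly, then destroys the actor and quits the game.
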(event `InputAxis|MoveForward`
  (params (AxisValue :type "Float (single-precision)"))
  (`self.AddMovementInput` (`self.GetActorForwardVector`) AxisValue))

(event `self.ReceiveAnyDamage`
  (params (Damage :type "Float (single-precision)") (DamageType :type "DamageType Object Reference") (InstigatedBy :type "Controller Object Reference") (DamageCauser :type "Actor Object Reference"))
  (bind _output_get (set `self.Energy` (- (`self.Energy`) Damage)))
  (if (<= _output_get 0.0)
    (`self.DisableInput` null)
    (bind _returnvalue (`|CreateWidget` "/Game/BP_WEnd.BP_WEnd_C"))
    (`UserWidget.AddToViewport` _returnvalue 0)
    (`KismetSystemLibrary.Delay` 3.0)
    (`Widget.RemoveFromParent` _returnvalue)
    (`KismetSystemLibrary.Delay` 1.0)
    (`self.K2_DestroyActor`)
    (`KismetSystemLibrary.QuitGame` null "Quit")))

(event `InputAxis|Turn`
  (params (AxisValue :type "Float (single-precision)"))
  (`self.AddControllerYawInput` AxisValue))

(event `InputAction|Run`
  (params (Key :type "Key Structure"))
  (bind _charactermovement (`self.CharacterMovement`))
  (:`Pressed`
    (set `CharacterMovementComponent.MaxWalkSpeed` 500.0 _charactermovement))
  (:`Released`
    (set `CharacterMovementComponent.MaxWalkSpeed` 300.0 _charactermovement)))

(event `self.ReceiveTick`
  (params (DeltaSeconds :type "Float (single-precision)")))

(event `InputAction|Shot`
  (params (Key :type "Key Structure"))
  (:`Pressed`
    (if (== (`MovementComponent.Velocity` (`self.CharacterMovement`)) (0.0 0.0 0.0) :`ErrorTolerance` 0.0)
      (set `self.IsShot` true)
      (`self.shot`)))
  (:`Released`
    (set `self.IsShot` false)))

(fn `shot`
  (`|SpawnActorFromClass` "/Game/BP_Bullet.BP_Bullet_C" (`SceneComponent.K2_GetComponentToWorld` (`self.Arrow1`)) "Undefined" "OverrideRootScale" null null))

(fn `UserConstructionScript`)